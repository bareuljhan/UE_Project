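; BP_Enemy is an enemy with health, a widget health bar and a simple reaction to being hit.
; AnyDamage records the instigator's pawn as Attacker if it is a Character, subtracts the damage from Health and refreshes the WB_EnemyHpBar widget.
; The enemy then snaps its rotation to face the Attacker.
; A final cast to BP_Player leads to no further logic, and no death handling is present.
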(event EventBeginPlay
  (Utilities|FlowControl|Sequence
    (:then_0
      (CallFunction|UpdateHealthBar))))

(event Game|Damage|EventAnyDamage
  (params (Damage :type Float%20%28single-precision%29) (DamageType :type Damage%20Type%20Object%20Reference) (InstigatedBy :type Controller%20Object%20Reference) (DamageCauser :type Actor%20Object%20Reference))
  (|SetDamage Damage InstigatedBy)
  (|SetRotateToAttacker)
  (Utilities|Casting|CastToBP_Player (Variables|Default|GetAttacker)))

(fn ConstructionScript)

(fn UpdateHealthBar
  (bind _aswb_enemy_hp_bar (Utilities|Casting|CastToWB_EnemyHpBar (UserInterface|GetUserWidgetObject (Variables|Default|GetHealthBar))))
  (Default|UpdateHealthBar _aswb_enemy_hp_bar (Variables|Default|GetHealth)))